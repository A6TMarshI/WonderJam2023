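; Cult character Blueprint that switches its animation between walking, praying, idling and talking.
; It drives the mesh's AIAnimMontage anim instance by setting its Action enum, starting in the walk state on BeginPlay.
; The Pray, Idle and Talk events each set their action, then start a timer by function name that calls GoWalk to restore walking after the given duration.
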(event EventBeginPlay
  (|CallParentFunction)
  (bind _asaianim_montage (Utilities|Casting|CastToAIAnimMontage (Components|SkeletalMesh|GetAnimInstance (Variables|Default|GetMeshComponent))))
  (Variables|/Game/WonderJam/Animation/AIAnimMontage.AIAnimMontage_C|Setaction _asaianim_montage "NewEnumerator1"))

(event EventOnPray
  (params (time :type Float%20%28single-precision%29))
  (bind _asaianim_montage (Utilities|Casting|CastToAIAnimMontage (Components|SkeletalMesh|GetAnimInstance (Variables|Default|GetMeshComponent))))
  (Variables|/Game/WonderJam/Animation/AIAnimMontage.AIAnimMontage_C|Setaction _asaianim_montage "NewEnumerator3")
  (Utilities|Time|SetTimerbyFunctionName 0 "GoWalk" time))

(event EventOnIdle
  (params (time :type Float%20%28single-precision%29))
  (bind _asaianim_montage (Utilities|Casting|CastToAIAnimMontage (Components|SkeletalMesh|GetAnimInstance (Variables|Default|GetMeshComponent))))
  (Variables|/Game/WonderJam/Animation/AIAnimMontage.AIAnimMontage_C|Setaction _asaianim_montage "NewEnumerator0")
  (Utilities|Time|SetTimerbyFunctionName 0 "GoWalk" time))

(event EventOnTalk
  (params (time :type Float%20%28single-precision%29))
  (bind _asaianim_montage (Utilities|Casting|CastToAIAnimMontage (Components|SkeletalMesh|GetAnimInstance (Variables|Default|GetMeshComponent))))
  (Variables|/Game/WonderJam/Animation/AIAnimMontage.AIAnimMontage_C|Setaction _asaianim_montage "NewEnumerator8")
  (Utilities|Time|SetTimerbyFunctionName 0 "GoWalk" time))

(fn ConstructionScript)

(fn GoWalk
  (bind _asaianim_montage (Utilities|Casting|CastToAIAnimMontage (Components|SkeletalMesh|GetAnimInstance (Variables|Default|GetMeshComponent))))
  (Variables|/Game/WonderJam/Animation/AIAnimMontage.AIAnimMontage_C|Setaction _asaianim_montage "NewEnumerator1"))